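; Player controller that lets a player spawn or despawn their character through the game mode.
; On BeginPlay it casts and caches the bpGameMode reference.
; Key 1 or gamepad Special Right calls OnPlayerSpawn, and key 2 or Special Left calls OnPlayerDespawn, each passing this controller.
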(event EventBeginPlay
  (bind _asbp_game_mode (Utilities|Casting|CastTobpGameMode (Game|GetGameMode)))
  (Variables|Default|SetGameModeRef _asbp_game_mode))

(event EventTick
  (params (DeltaSeconds :type Float%20%28single-precision%29)))

(event Input|GamepadEvents|GamepadSpecialLeft
  (params (Key :type Key%20Structure))
  (:Pressed
    (Default|OnPlayerDespawn (Variables|Default|GetGameModeRef) self)))

(event Input|GamepadEvents|GamepadSpecialRight
  (params (Key :type Key%20Structure))
  (:Pressed
    (Default|OnPlayerSpawn (Variables|Default|GetGameModeRef) self)))

(event Input|KeyboardEvents|1
  (params (Key :type Key%20Structure))
  (:Pressed
    (Default|OnPlayerSpawn (Variables|Default|GetGameModeRef) self)))

(event Input|KeyboardEvents|2
  (params (Key :type Key%20Structure))
  (:Pressed
    (Default|OnPlayerDespawn (Variables|Default|GetGameModeRef) self)))

(fn ConstructionScript)