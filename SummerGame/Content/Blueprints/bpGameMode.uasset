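; Game mode for local multiplayer on a shared camera, creating players at BeginPlay by looping over the count of PlayerStart actors.
; Spawn and despawn events swap a player between the character and placeholder pawns through a common Spawn function.
; Spawn destroys the current valid pawn, spawns the replacement at GetRandomSpawnPoint's transform, possesses it and sets the view target to SharedCamera.
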(event Custom|OnPlayerSpawn
  (params (PlayerController :type Player%20Controller%20Object%20Reference))
  (CallFunction|Spawn PlayerController "/Game/Blueprints/bpPlayerCharacter.bpPlayerCharacter_C"))

(event Custom|OnPlayerDespawn
  (params (PlayerController :type Player%20Controller%20Object%20Reference))
  (CallFunction|Spawn PlayerController "/Game/Blueprints/bpPlayerPlaceholder.bpPlayerPlaceholder_C"))

(event EventBeginPlay
  (bind _outactors (Actor|GetAllActorsOfClass "/Script/Engine.PlayerStart"))
  (bind _output_get (Variables|Default|SetSpawnPoints _outactors))
  (for _index (range 0 (Utilities|Array|Length _output_get))
    (Class|GameplayStatics|CreatePlayer _index)))

(fn ConstructionScript)

(fn Spawn
  (params (PlayerController :type Player%20Controller%20Object%20Reference) (SpawnType :type Actor%20Class%20Reference))
  (bind _returnvalue (Pawn|GetControlledPawn PlayerController))
  (Utilities|IsValid _returnvalue
    (:Is%20Valid
      (Actor|DestroyActor _returnvalue)
      (bind _returnvalue_2 (Game|SpawnActorfromClass SpawnType (Utilities|GetRandomSpawnPoint) "Undefined" 0 0))
      (bind _aspawn (Utilities|Casting|CastToPawn _returnvalue_2))
      (Pawn|Possess PlayerController _aspawn)
      (Game|Player|SetViewTargetwithBlend PlayerController (Variables|Default|GetSharedCamera) 0.0 "VTBlend_Linear" 0.0 false))))